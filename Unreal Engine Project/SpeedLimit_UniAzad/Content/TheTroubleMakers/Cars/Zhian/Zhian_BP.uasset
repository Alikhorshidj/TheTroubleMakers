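; Zhian_BP is a drivable car Blueprint with throttle, steering, mouse-orbit camera and openable doors.
; Input axes feed the vehicle movement component and rotate the spring arm; the brake action releases the handbrake when pressed and engages it when released.
; FlipFlops play or reverse per-door timelines that update door angle variables.
; Tick stores the larger absolute steer angle of the first two wheels as an unsigned SteeringAngle.
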(event EventBeginPlay)

(event Collision|EventActorBeginOverlap
  (params (OtherActor :type Actor%20Object%20Reference)))

(event EventTick
  (params (DeltaSeconds :type Float%20%28single-precision%29))
  (CallFunction|SteeringWheelUpdate))

(event Input|ActionEvents|InputActionVehicleBreak
  (params (Key :type Key%20Structure :default "None"))
  (bind _vehiclemovement (Variables|Default|GetVehicleMovement))
  (:Pressed
    (Class|WheeledVehicleMovementComponent|SetHandbrakeInput _vehiclemovement false))
  (:Released
    (Class|WheeledVehicleMovementComponent|SetHandbrakeInput _vehiclemovement true)))

(event Input|ActionEvents|InputActionLeftDoorTrigger
  (params (Key :type Key%20Structure :default "None"))
  ;[1 1 1] Door Functinality
  (:Pressed
    (Utilities|FlowControl|FlipFlop
      (:A
        (bind _door_angle (Timeline|Left%20Door Play)
          (:Update
            (Variables|Default|SetLeft%20Door%20Angle _door_angle))))
      (:B
        (Timeline|Left%20Door Reverse)))))

(event Input|ActionEvents|InputActionRightDoorTrigger
  (params (Key :type Key%20Structure :default "None"))
  ;[1 1 1] Door Functinality
  (:Pressed
    (Utilities|FlowControl|FlipFlop
      (:A
        (bind _door_angle (Timeline|Right%20Door Play)
          (:Update
            (Variables|Default|SetRight%20Door%20Angle _door_angle))))
      (:B
        (Timeline|Right%20Door Reverse)))))

(event Input|AxisEvents|InputAxisThrottle
  (params (AxisValue :type Float%20%28single-precision%29))
  (Class|WheeledVehicleMovementComponent|SetThrottleInput (Variables|Default|GetVehicleMovement) AxisValue))

(event Input|AxisEvents|InputAxisSteering
  (params (AxisValue :type Float%20%28single-precision%29))
  (Class|WheeledVehicleMovementComponent|SetSteeringInput (Variables|Default|GetVehicleMovement) AxisValue))

(event Input|MouseEvents|MouseX
  (params (AxisValue :type Float%20%28single-precision%29))
  (Transformation|AddRelativeRotation (Variables|Default|GetSpringArm) (Math|Rotator|MakeRotator 0.0 0.0 AxisValue) false false))

(event Input|MouseEvents|MouseY
  (params (AxisValue :type Float%20%28single-precision%29))
  (Transformation|AddRelativeRotation (Variables|Default|GetSpringArm) (Math|Rotator|MakeRotator 0.0 AxisValue 0.0) false false))

(fn ConstructionScript)

(fn SteeringWheelUpdate
  (bind _vehiclemovement (Variables|Default|GetVehicleMovement))
  (bind _wheels (Variables|/Script/PhysXVehicles.WheeledVehicleMovementComponent|GetWheels _vehiclemovement))
  (bind _output (Utilities|Array|Get(acopy) _wheels))
  (bind _output_2 (Utilities|Array|Get(acopy) _wheels 1))
  (bind _returnvalue (Class|VehicleWheel|GetSteerAngle _output_2))
  (bind _returnvalue_2 (Class|VehicleWheel|GetSteerAngle _output))
  (bind _returnvalue_3 (Math|Float|Absolute(Float) _returnvalue))
  (bind _returnvalue_4 (Math|Float|Absolute(Float) _returnvalue_2))
  (Variables|Default|SetSteering%20Angle (Math|Float|SelectFloat _returnvalue_4 _returnvalue_3 (> _returnvalue_4 _returnvalue_3))))